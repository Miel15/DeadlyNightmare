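; Speed power-up pickup Blueprint that gives the player a temporary speed boost.
; While the Existe flag is set, Tick checks distance to the player character instead of using overlap events.
; Within range it calls SpeedPowerUp on MyCharacter once, guarded by Used, and hides a component rather than destroying the actor.
; After a fixed Delay it prints a debug message and calls SpeedPowerUpEnd.
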(event EventTick
  (params (DeltaSeconds :type Float%20%28single-precision%29))
  (if (Variables|Default|GetExiste)
    (if (<= (Math|Vector|VectorLength (- (Transformation|GetWorldLocation) (Transformation|GetWorldLocation (Game|GetPlayerCharacter 0)))) 1e+02)
      (bind _asmy_character (Utilities|Casting|CastToMyCharacter (Pawn|GetControlledPawn (Game|GetPlayerController 0)))
        (:then
          (if (not (Variables|Default|GetUsed))
            (Default|SpeedPowerUp _asmy_character)
            (Rendering|SetVisibility false false)
            (Variables|Default|SetUsed true)
            (Utilities|FlowControl|Delay 15.0)
            (Development|PrintString "Acabo")
            (Default|SpeedPowerUpEnd _asmy_character)))
        (:CastFailed
          (Development|PrintString "cast failed"))))))

(fn ConstructionScript)