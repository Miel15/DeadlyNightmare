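; Enemy-like Blueprint that loses health on hits and chases via SimpleMoveToActor, with the player controller, not its pawn, as goal.
; Any Box1 overlap subtracts fixed damage and prints Health, without checking for bullets as its comment intends.
; Tick shares the move and death check, destroying components once Health reaches MinLife.
; The death animation is only a comment, and Perseguir and the construction script are empty.
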(event OnComponentBeginOverlap(Box1)
  (params (OtherActor :type Actor%20Object%20Reference) (OtherComp :type Primitive%20Component%20Object%20Reference) (OtherBodyIndex :type Integer) (bFromSweep :type Boolean) (SweepResult :type Hit%20Result%20Structure%20%28by%20ref%29))
  ;[1 1 1] Lógica para que las balas bajen vida
  (Variables|Default|SetHealth (- (Variables|Default|GetHealth) 1e+01))
  (Development|PrintString (Utilities|String|ToString(Float) (Variables|Default|GetHealth)))
  (AI|Navigation|SimpleMovetoActor (Pawn|GetController) (Game|GetPlayerController 0))
  (if (<= (Variables|Default|GetHealth) (Variables|Default|GetminLife))
    ;[1 1 1] Aqui debe suceder la animación de muerte
    (Components|DestroyComponent)
    (Components|DestroyComponent)
    (Components|DestroyComponent)
    (Components|DestroyComponent)))

(event EventTick
  (params (DeltaSeconds :type Float%20%28single-precision%29))
  (AI|Navigation|SimpleMovetoActor (Pawn|GetController) (Game|GetPlayerController 0))
  ;[1 1 1] Lógica para que las balas bajen vida
  (if (<= (Variables|Default|GetHealth) (Variables|Default|GetminLife))
    ;[1 1 1] Aqui debe suceder la animación de muerte
    (Components|DestroyComponent)
    (Components|DestroyComponent)
    (Components|DestroyComponent)
    (Components|DestroyComponent)))

(fn ConstructionScript)

(fn Perseguir)