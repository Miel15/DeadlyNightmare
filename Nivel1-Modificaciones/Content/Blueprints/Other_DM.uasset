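; Enemy Blueprint that chases the player at close range and loses health when hit by projectiles.
; Box overlaps compare the other actor's class to MyProjectile's, then subtract health.
; Tick checks player distance while alive, only printing a damage message at the nearest range, and shares the overlap's move-and-death chain, which targets the player controller and destroys components at minimum health.
; The death animation is only a comment, and Perseguir is empty.
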(event OnComponentBeginOverlap(Box1)
  (params (OtherActor :type Actor%20Object%20Reference) (OtherComp :type Primitive%20Component%20Object%20Reference) (OtherBodyIndex :type Integer) (bFromSweep :type Boolean) (SweepResult :type Hit%20Result%20Structure%20%28by%20ref%29))
  (bind _asmy_projectile (Utilities|Casting|CastToMyProjectile (Variables|Default|Gettest)))
  ;[1 1 1] Lógica para que las balas bajen vida
  (if (== (Utilities|GetClass OtherActor) (Utilities|GetClass _asmy_projectile))
    (Variables|Default|SetHealth (- (Variables|Default|GetHealth) 1e+01))
    (Development|PrintString (Utilities|String|ToString(Float) (Variables|Default|GetHealth)))
    (AI|Navigation|SimpleMovetoActor (Pawn|GetController) (Game|GetPlayerController 0))
    (if (<= (Variables|Default|GetHealth) (Variables|Default|GetminLife))
      (Variables|Default|SetExiste false)
      ;[1 1 1] Aqui debe suceder la animación de muerte
      (Components|DestroyComponent)
      (Components|DestroyComponent)
      (Components|DestroyComponent)
      (Components|DestroyComponent))))

(event EventTick
  (params (DeltaSeconds :type Float%20%28single-precision%29))
  (bind _returnvalue (Game|GetPlayerCharacter 0))
  (bind _returnvalue_2 (Transformation|GetWorldLocation))
  (bind _returnvalue_3 (Transformation|GetWorldLocation _returnvalue))
  (bind _returnvalue_4 (- _returnvalue_2 _returnvalue_3))
  (bind _returnvalue_5 (Math|Vector|VectorLength _returnvalue_4))
  ;[1 1 1] para detectar distancias
  (if (Variables|Default|GetExiste)
    (if (<= _returnvalue_5 6e+02)
      (if (<= _returnvalue_5 3e+02)
        (Development|PrintString "daño"))
      (AI|Navigation|SimpleMovetoActor (Pawn|GetController) (Game|GetPlayerController 0))
      ;[1 1 1] Lógica para que las balas bajen vida
      (if (<= (Variables|Default|GetHealth) (Variables|Default|GetminLife))
        (Variables|Default|SetExiste false)
        ;[1 1 1] Aqui debe suceder la animación de muerte
        (Components|DestroyComponent)
        (Components|DestroyComponent)
        (Components|DestroyComponent)
        (Components|DestroyComponent)))))

(fn ConstructionScript)

(fn Perseguir)